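; Enemy spawner actor that periodically creates BP_Enemy instances in the level.
; On BeginPlay it caches every BP_Spawn actor in the level as the list of spawn locations.
; Tick accumulates time and, once the delay is reached, spawns an enemy at a randomly chosen point's transform, adjusting for collisions but always spawning, then resets the timer.
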(event EventBeginPlay
  (bind _outactors (Actor|GetAllActorsOfClass "/Game/MS/Blueprint/BP_Spawn.BP_Spawn_C"))
  (Variables|Default|SetSpawnList _outactors) ; 스폰위치 배열에 저장
)

(event Collision|EventActorBeginOverlap
  (params (OtherActor :type Actor%20Object%20Reference)))

(event EventTick
  (params (DeltaSeconds :type Float%20%28single-precision%29))
  (bind _spawnlist (Variables|Default|GetSpawnList))
  (bind _output_get (Variables|Default|SetCurrentTime (+ DeltaSeconds (Variables|Default|GetCurrentTime))))
  (if (>= _output_get (Variables|Default|GetDelayTime))
    (Game|SpawnActorfromClass "/Game/EB/Blueprints/BP_Enemy.BP_Enemy_C" (Transformation|GetWorldTransform (Variables|/Script/Engine.Actor|GetRootComponent (Utilities|Array|Get(acopy) _spawnlist (Math|Random|RandomInteger (Utilities|Array|Length _spawnlist))))) "AdjustIfPossibleButAlwaysSpawn" "MultiplyWithRoot" 0 0)
    (Variables|Default|SetCurrentTime 0.0)))

(fn ConstructionScript)